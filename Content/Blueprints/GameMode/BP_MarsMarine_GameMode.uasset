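; Game mode for Mars Marine that runs endless waves of alien spiders.
; Each wave scales the previous spider count by a difficulty multiplier, then a looping timer spawns BP_Alien at random TargetPoints until the count runs out.
; From wave two onward, spawned spiders get a set higher health and double scale.
; RegisterSpiderDead removes spiders from the tracked array and starts the next wave after a delay once none remain.
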(event Custom|SpawnSpider
  (bind _returnvalue (CallFunction|EnemySpawn))
  (Utilities|Array|Add (Variables|Default|GetSpiderArray) _returnvalue)
  (bind _result (Math|Integer|DecrementInt (Variables|Default|GetSpiderRemainingToSpawn))
    (:%20%20
      (bind _output_get (Variables|Default|SetSpiderRemainingToSpawn _result))
      (if (== _output_get 0)
        (Utilities|Time|ClearTimerbyFunctionName 0 "SpawnSpider")))))

(event Custom|EndWave
  (Utilities|FlowControl|Delay 2.0)
  (CallFunction|StartNewWave))

(event EventBeginPlay
  (Utilities|FlowControl|Delay 2.0)
  (CallFunction|StartNewWave))

(fn ConstructionScript)

(fn EnemySpawn
  (bind _outactors (Actor|GetAllActorsOfClass "/Script/Engine.TargetPoint"))
  (bind _returnvalue (Game|SpawnActorfromClass "/Game/Blueprints/AI/BP_Alien.BP_Alien_C" (Transformation|GetActorTransform (Utilities|Array|Get(acopy) _outactors (Math|Random|RandomIntegerinRange 0 (Utilities|Array|LastIndex _outactors)))) "Undefined" 0 0))
  (if (>= (Variables|Default|GetWaveNumber) 2)
    (bind _output_get (Variables|Default|SetSpawnedMoreHPSpider _returnvalue))
    (Variables|/Game/Blueprints/AI/BP_Alien.BP_Alien_C|SetHealthSpider _output_get 1.5e+02)
    (Transformation|SetActorScale3D _output_get (* (Transformation|GetActorScale3D _output_get) 2.0)))
  (return _returnvalue))

(fn RegisterSpiderDead
  (params (Item :type BP%20Alien%20Object%20Reference%20%28by%20ref%29))
  (bind _spiderarray (Variables|Default|GetSpiderArray))
  (Utilities|Array|RemoveItem _spiderarray Item)
  (if (and (== (Utilities|Array|Length _spiderarray) 0) (== (Variables|Default|GetSpiderRemainingToSpawn) 0))
    (CallFunction|EndWave)))

(fn StartNewWave
  (Math|Integer|IncrementInt (Variables|Default|GetWaveNumber)
    (:%20%20
      (CallFunction|DifficultWave)
      (Utilities|Time|SetTimerbyFunctionName 0 "SpawnSpider" 2.0 true))))

(fn DifficultWave
  (bind _output_get (Variables|Default|SetSpiderRemainingToSpawn (Math|Float|Round (* (Variables|Default|GetSpiderLastLiczba) (Variables|Default|GetDifficult%20Lvl)))))
  (Variables|Default|SetSpiderLastLiczba _output_get))