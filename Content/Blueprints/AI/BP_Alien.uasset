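; BP_Alien is a spider enemy that chases the player and plays an attack montage when close to the marine.
; AIMoveTo repeats after a short delay on success or failure, while Tick checks range and pauses movement during the attack.
; AnyDamage lowers health; at zero the spider is destroyed, increments the marine's kill count and registers its death with BP_MarsMarine_GameMode.
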(event EventBeginPlay
  (if (not (Variables|Default|GetDeadSpider))
    (AI|AIMoveTo self "0, 0, 0" (Game|GetPlayerCharacter 0) 5.0 false :!label _label
      (:OnSuccess
        _)
      (:OnFail
        _))
    (Utilities|FlowControl|Delay 0.2)
    (goto _label)))

(event Game|Damage|EventAnyDamage
  (params (Damage :type Float%20%28single-precision%29) (DamageType :type Damage%20Type%20Object%20Reference) (InstigatedBy :type Controller%20Object%20Reference) (DamageCauser :type Actor%20Object%20Reference))
  ;[0.156 0.8194 1] Obrazenia dla pająka :(
  (CallFunction|IfAnyDamagetoSpiderThenDie Damage)
  (if (Variables|Default|GetDeadSpider)
    (Actor|DestroyActor)
    (CallFunction|ZwiększanieLiczbyKill)))

(event EventTick
  (params (DeltaSeconds :type Float%20%28single-precision%29))
  ;[1 0.2078 0.0478] Attack Spider :)
  (if (not (Variables|Default|GetDeadSpider))
    (if (and (CallFunction|ISAttackRANGE) (not (CallFunction|IsATTACKING?)))
      (Components|Activation|Deactivate (Variables|Character|GetCharacterMovement))
      (Animation|Montage|PlayMontage (Variables|Character|GetMesh) "/Game/Characters/Enemy_Great_Spider/Animations/spiderattack.spiderattack" 2.0
        (:OnCompleted
          (Components|Activation|Activate (Variables|Character|GetCharacterMovement) false))))))

(fn ConstructionScript)

(fn ISAttackRANGE
  (bind _asbp_marine (Utilities|Casting|CastToBP_Marine (Game|Player|GetPlayerPawn 0)))
  (return (< (Transformation|GetDistanceTo _asbp_marine) 1e+02)))

(fn IsATTACKING?
  (return (Animation|Montage|MontageIsPlaying (Components|SkeletalMesh|GetAnimInstance (Variables|Character|GetMesh)) "/Game/Characters/Enemy_Great_Spider/Animations/spiderattack.spiderattack")))

(fn IfAnyDamagetoSpiderThenDie
  (params (Damage :type Float%20%28single-precision%29))
  (bind _output_get (Variables|Default|SetHealthSpider (- (Variables|Default|GetHealthSpider) Damage)))
  (if (== (Math|Float|Clamp(Float) _output_get 0.0 1e+02) 0.0)
    (bind _output_get_2 (Variables|Default|SetDeadSpider true))
    (return _output_get_2)))

(fn ZwiększanieLiczbyKill
  (bind _asbp_marine (Utilities|Casting|CastToBP_Marine (Game|GetPlayerCharacter 0)))
  (Variables|Default|SetAs%20BP%20Marine _asbp_marine)
  (bind _result (Math|Integer|IncrementInt (Variables|/Game/Blueprints/Pawns/BP_Marine.BP_Marine_C|GetKills (Variables|Default|GetAs%20BP%20Marine)))
    (:%20%20
      (Variables|/Game/Blueprints/Pawns/BP_Marine.BP_Marine_C|SetKills (Variables|Default|GetAs%20BP%20Marine) _result)
      (bind _asbp_mars_marine_game_mode (Utilities|Casting|CastToBP_MarsMarine_GameMode (Game|GetGameMode)))
      (Default|RegisterSpiderDead _asbp_mars_marine_game_mode self))))